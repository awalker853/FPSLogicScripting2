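; DamagedPlaceholder is a damageable placeholder target that disappears when its health runs out.
; The AnyDamage event passes the damage to TakeDamageFromSource, which subtracts it from Health and clamps the result between zero and MaxHealth.
; At zero health it hides the SphereTarget component and disables its collision, leaving the actor itself in place.
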(event `self.ReceiveAnyDamage`
  (params (Damage :type "Float (single-precision)") (DamageType :type "DamageType Object Reference") (InstigatedBy :type "Controller Object Reference") (DamageCauser :type "Actor Object Reference"))
  (`self.TakeDamageFromSource` Damage))

(fn `TakeDamageFromSource`
  (params (Damage :type "Float (double-precision)"))
  (bind _spheretarget (`self.SphereTarget`))
  (bind _output_get (set `self.Health` (`KismetMathLibrary.FClamp` (- (`self.Health`) Damage) 0.0 (`self.MaxHealth`))))
  (if (== _output_get 0.0)
    (`SceneComponent.SetVisibility` _spheretarget false false)
    (`PrimitiveComponent.SetCollisionEnabled` _spheretarget "NoCollision")))

(fn `UserConstructionScript`)