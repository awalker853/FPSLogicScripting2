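; First-person player character that handles movement, look, jumping and rifle combat.
; On BeginPlay it spawns BP_Rifle, stores it as the equipped gun and attaches it to GunLocation.
; Holding the shoot axis fires from the camera's forward vector, with a CanPlayerShoot flag and Delay enforcing the gun's fire rate.
; Empty ammo or the Reload input triggers a timed reload to a hardcoded magazine size, with debug prints for ammo and reloading.
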(event `InputAction|Jump`
  (params (Key :type "Key Structure"))
  (:`Pressed`
    (`self.Jump`)))

(event `InputAxis|MoveForwardBack`
  (params (AxisValue :type "Float (single-precision)"))
  (`self.AddMovementInput` (`self.GetActorForwardVector`) AxisValue))

(event `InputAxis|LookLeftRight`
  (params (AxisValue :type "Float (single-precision)"))
  (`self.AddControllerYawInput` AxisValue))

(event `InputAxis|MoveRightLeft`
  (params (AxisValue :type "Float (single-precision)"))
  (`self.AddMovementInput` (`self.GetActorRightVector`) AxisValue))

(event `InputAxis|LookUpDown`
  (params (AxisValue :type "Float (single-precision)"))
  (`self.AddControllerPitchInput` AxisValue))

(event `self.ReceiveBeginPlay`
  (bind _returnvalue (`|SpawnActorFromClass` "/Game/Blueprints/BP_Rifle.BP_Rifle_C" (`KismetMathLibrary.MakeTransform` (0.0 0.0 0.0)) "Undefined" "OverrideRootScale" null null))
  (bind _output_get (set `self.CurrentlyEquippedGun` _returnvalue))
  (`self.K2_AttachToComponent` _output_get (`self.GunLocation`) "None" "SnapToTarget" "SnapToTarget" "KeepRelative" true))

(event `InputAxis|ShootAxis`
  (params (AxisValue :type "Float (single-precision)"))
  (bind _fpscamera (`self.FPSCamera`))
  (bind _currentlyequippedgun (`self.CurrentlyEquippedGun`))
  (bind _returnvalue (`SceneComponent.K2_GetComponentLocation` _fpscamera))
  (if (and (== AxisValue 1) (`self.CanPlayerShoot`))
    (`/Game/Blueprints/BP_GunTemplate.Shoot` (`self.CurrentlyEquippedGun`) _returnvalue (+ (* (`SceneComponent.GetForwardVector` _fpscamera) (`/Game/Blueprints/BP_GunTemplate.MaxBulletDistance` (`self.CurrentlyEquippedGun`))) _returnvalue))
    (bind _output_get (set `/Game/Blueprints/BP_GunTemplate.Ammo` (- (`/Game/Blueprints/BP_GunTemplate.Ammo` _currentlyequippedgun) 1.0) _currentlyequippedgun))
    (`KismetSystemLibrary.PrintString` (`KismetStringLibrary.Conv_DoubleToString` _output_get))
    (set `self.CanPlayerShoot` false)
    (`KismetSystemLibrary.Delay` (`/Game/Blueprints/BP_GunTemplate.RateOfFire` (`self.CurrentlyEquippedGun`)))
    (if (== (`/Game/Blueprints/BP_GunTemplate.Ammo` (`self.CurrentlyEquippedGun`)) 0.0)
      (`KismetSystemLibrary.PrintString` "Reloading")
      (`KismetSystemLibrary.Delay` 2.0)
      (`self.ReloadFnct`)
      (set `self.CanPlayerShoot` true)
      (else
        (set `self.CanPlayerShoot` true)))))

(event `InputAction|Reload`
  (params (Key :type "Key Structure"))
  (:`Pressed`
    (`KismetSystemLibrary.PrintString` "Reloading")
    (set `self.CanPlayerShoot` false)
    (`KismetSystemLibrary.Delay` 2.0)
    (`self.ReloadFnct`)
    (set `self.CanPlayerShoot` true)))

(fn `ReloadFnct`
  (set `/Game/Blueprints/BP_GunTemplate.Ammo` 30.0 (`self.CurrentlyEquippedGun`)))

(fn `UserConstructionScript`)